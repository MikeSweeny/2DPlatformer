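; Two-way teleporter that moves the player character between two box volumes, Box and Box1.
; Entering either box while Reset is true teleports the character to the other box's location with zero rotation.
; Leaving either box sets Reset to true, but nothing in these graphs clears it, so the flag does not block re-teleporting on arrival once set.
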(event OnComponentBeginOverlap(Box)
  (params (OverlappedComponent :type Primitive%20Component%20Object%20Reference) (OtherActor :type Actor%20Object%20Reference) (OtherComp :type Primitive%20Component%20Object%20Reference) (OtherBodyIndex :type Integer) (bFromSweep :type Boolean) (SweepResult :type Hit%20Result%20Structure%20%28by%20ref%29))
  (bind _returnvalue (Game|Player|GetPlayerPawn 0))
  (if (== OtherActor _returnvalue)
    (if (Variables|Default|Getreset)
      (bind _ascharacter (Utilities|Casting|CastToCharacter _returnvalue))
      (bind _returnvalue_2 (Transformation|Teleport _ascharacter (Transformation|GetWorldLocation (Variables|Default|GetBox1)) "0, 0, 0")))))

(event OnComponentBeginOverlap(Box1)
  (params (OverlappedComponent :type Primitive%20Component%20Object%20Reference) (OtherActor :type Actor%20Object%20Reference) (OtherComp :type Primitive%20Component%20Object%20Reference) (OtherBodyIndex :type Integer) (bFromSweep :type Boolean) (SweepResult :type Hit%20Result%20Structure%20%28by%20ref%29))
  (bind _returnvalue (Game|Player|GetPlayerPawn 0))
  (if (== OtherActor _returnvalue)
    (if (Variables|Default|Getreset)
      (bind _ascharacter (Utilities|Casting|CastToCharacter _returnvalue))
      (bind _returnvalue_2 (Transformation|Teleport _ascharacter (Transformation|GetWorldLocation (Variables|Default|GetBox)) "0, 0, 0")))))

(event OnComponentEndOverlap(Box)
  (params (OverlappedComponent :type Primitive%20Component%20Object%20Reference) (OtherActor :type Actor%20Object%20Reference) (OtherComp :type Primitive%20Component%20Object%20Reference) (OtherBodyIndex :type Integer))
  (if (== OtherActor (Game|Player|GetPlayerPawn 0))
    (Variables|Default|Setreset true)))

(event OnComponentEndOverlap(Box1)
  (params (OverlappedComponent :type Primitive%20Component%20Object%20Reference) (OtherActor :type Actor%20Object%20Reference) (OtherComp :type Primitive%20Component%20Object%20Reference) (OtherBodyIndex :type Integer))
  (if (== OtherActor (Game|Player|GetPlayerPawn 0))
    (Variables|Default|Setreset true)))

(fn ConstructionScript)