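; Moving platform actor that follows a Timeline-driven offset from its starting location, presumably along X as the asset name suggests.
; A custom trigger event, not called within this Blueprint, caches the actor location, waits StartPlat seconds, then sets the Start flag.
; While Start is true, Tick calls Play on the Timeline every frame, and its updates add the track value to the cached location without sweeping.
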(event Custom|CustomEvent
  ;[1 1 1] Start Trigger
  (Variables|Default|SetLocationOnPlay (Transformation|GetActorLocation))
  (Utilities|FlowControl|Delay (Variables|Default|GetStartPlat))
  (Variables|Default|SetStart true))

(event Collision|EventActorBeginOverlap
  (params (OtherActor :type Actor%20Object%20Reference)))

(event EventTick
  (params (DeltaSeconds :type Float%20%28single-precision%29))
  (if (Variables|Default|GetStart)
    (Utilities|FlowControl|Sequence
      (:then_0
        (bind _newtrack_0 (Timeline|Timeline_0 Play)
          (:Update
            (Transformation|SetActorLocation (+ _newtrack_0 (Variables|Default|GetLocationOnPlay)) false false)))))))

(event EventBeginPlay)

(fn ConstructionScript)