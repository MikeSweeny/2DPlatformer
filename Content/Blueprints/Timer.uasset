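; Timer Blueprint that keeps an elapsed minutes and seconds count and shows it as on-screen debug text.
; Tick counts frames and treats every 60 as one second, so its pace follows frame rate rather than delta time.
; Each such step prints Min:Sec in dark green, then increments Sec, which rolls into Min upon reaching 59, not 60.
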(event EventTick
  (params (DeltaSeconds :type Float%20%28single-precision%29))
  (Math|Integer|IncrementInt (Variables|Default|Getframes)
    (:%20%20
      (if (== (Variables|Default|Getframes) 60)
        (Variables|Default|Setframes 0)
        (Development|PrintString (Utilities|String|Append (Utilities|String|ToString(Integer) (Variables|Default|GetMin)) " : " (Utilities|String|ToString(Integer) (Variables|Default|GetSec))) true true "(R=0.019166,G=0.131944,B=0.000000,A=1.000000)")
        (Math|Integer|IncrementInt (Variables|Default|GetSec)
          (:%20%20
            (if (== (Variables|Default|GetSec) 59)
              (Variables|Default|SetSec (- (Variables|Default|GetSec) 59))
              (Math|Integer|IncrementInt (Variables|Default|GetMin)))))))))

(fn ConstructionScript)