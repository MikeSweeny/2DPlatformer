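; PointPowerup is a pickup actor that awards the player a point on touch.
; On overlap with player pawn 0, it increments Score on the GlobalInstance game instance, so the total lives outside the level's actors.
; It then prints the new score as a colored on-screen string and destroys itself.
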(event Collision|EventActorBeginOverlap
  (params (OtherActor :type Actor%20Object%20Reference))
  (if (== OtherActor (Game|Player|GetPlayerPawn 0))
    (bind _asglobal_instance (Utilities|Casting|CastToGlobalInstance (Game|GetGameInstance)))
    (bind _asglobal_instance_2 (Utilities|Casting|CastToGlobalInstance (Game|GetGameInstance)))
    (bind _output_get (Variables|/Game/Blueprints/GlobalInstance.GlobalInstance_C|SetScore _asglobal_instance (+ (Variables|/Game/Blueprints/GlobalInstance.GlobalInstance_C|GetScore _asglobal_instance_2) 1)))
    (Development|PrintString (Utilities|String|ToString(Integer) _output_get) true true "(R=1.000000,G=0.000000,B=0.082829,A=1.000000)")
    (Actor|DestroyActor)))

(fn ConstructionScript)