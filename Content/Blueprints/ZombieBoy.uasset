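; ZombieBoy is a 2D flipbook character that animates and turns according to its movement.
; Each tick it switches the sprite between Walk and Idle flipbooks based on whether velocity is non-zero.
; It sets control rotation yaw to face the direction of horizontal velocity.
; When horizontal velocity is zero, the BisMovingRight flag picks the facing, though nothing in this Blueprint sets that flag.
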(event Custom|Update%20Animation
  (Sprite|SetFlipbook (Variables|Default|GetSprite) (select (> (Math|Vector|VectorLength (Transformation|GetVelocity)) 0.0) "/Game/Blueprints/Enemies/Zombie/male/Walk/Walk.Walk" "/Game/2DSideScrollerBP/CleanedUP/Characters/Zombie_Male/Idle/Flipbook/Idle.Idle")))

(event EventBeginPlay)

(event Collision|EventActorBeginOverlap
  (params (OtherActor :type Actor%20Object%20Reference)))

(event EventTick
  (params (DeltaSeconds :type Float%20%28single-precision%29))
  (CallFunction|UpdateAnimation)
  (Math|Float|CompareFloat (.X (Math|Vector|BreakVector (Variables|/Script/Engine.MovementComponent|GetVelocity (Pawn|GetMovementComponent)))) 0.0
    (:>
      (Pawn|SetControlRotation (Pawn|GetController) (Math|Rotator|MakeRotator 0.0 0.0 0.0) :!label _label))
    (:==
      (if (Variables|Default|GetbisMovingRight)
        (goto _label)
        (else
          (Pawn|SetControlRotation (Pawn|GetController) (Math|Rotator|MakeRotator 0.0 0.0 1.8e+02) :!label _label_2))))
    (:<
      (goto _label_2))))

(fn ConstructionScript)