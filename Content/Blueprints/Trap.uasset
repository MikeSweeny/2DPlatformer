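; Trap Blueprint that switches between acting and stopping based on whether its location is on screen for the first player.
; Each Tick, ScreenCheck projects the actor's location to screen space and tests it against the viewport bounds, calling Act when inside and StopAction otherwise.
; Act and StopAction are empty stubs, so this asset defines only the visibility gate, with no trap behavior.
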(event EventBeginPlay)

(event Collision|EventActorBeginOverlap
  (params (OtherActor :type Actor%20Object%20Reference)))

(event EventTick
  (params (DeltaSeconds :type Float%20%28single-precision%29))
  (bind _returnvalue (CallFunction|ScreenCheck))
  (if _returnvalue
    (CallFunction|Act)
    (else
      (CallFunction|StopAction))))

(fn ConstructionScript)

(fn ScreenCheck
  (bind _returnvalue (Game|GetPlayerController 0))
  (bind _returnvalue_2 (Transformation|GetActorLocation))
  (bind _returnvalue_3 (Viewport|GetViewportSize))
  (bind _screenlocation (Class|PlayerController|ProjectWorldLocationtoScreen _returnvalue _returnvalue_2 false))
  (return (Math|Boolean|ANDBoolean (> (.x _screenlocation) 0.0) (> (.y _screenlocation) 0.0) (< (.x _screenlocation) (.x _returnvalue_3)) (< (.y _screenlocation) (.y _returnvalue_3)))))

(fn Act)

(fn StopAction)