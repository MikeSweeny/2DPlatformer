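; Spikes actor that moves vertically on a repeating cycle once its Act event is triggered.
; BeginPlay caches the Box's world location as the base point.
; The Oscillate timeline's Wave track lerps the root between that point and 200 units above it, without sweep.
; On finish the timeline restarts in the same direction, so the motion loops; the file has no overlap or damage logic.
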(event EventBeginPlay
  (|CallParentFunction)
  (bind _output_get (Variables|Default|Setinit%20Location (Transformation|GetWorldLocation (Variables|Default|GetBox)))))

(event Collision|EventActorBeginOverlap
  (params (OtherActor :type Actor%20Object%20Reference))
  (|CallParentFunction OtherActor) ; This node is disabled and will not be called.\nDrag off pins to build functionality.
)

(event EventTick
  (params (DeltaSeconds :type Float%20%28single-precision%29))
  (|CallParentFunction DeltaSeconds))

(event EventAct
  (bind (_direction _wave) (Timeline|Oscillate Play)
    (:Update
      (Transformation|SetWorldLocation (Variables|Default|GetDefaultSceneRoot) (Math|Vector|Lerp(Vector) (stale EventBeginPlay _output_get) (Math|Vector|MakeVector (.X (Math|Vector|BreakVector (stale EventBeginPlay _output_get))) (.Y (Math|Vector|BreakVector (stale EventBeginPlay _output_get))) (+ (.Z (Math|Vector|BreakVector (stale EventBeginPlay _output_get))) 2e+02)) _wave) false false))
    (:Finished
      (switch Utilities|FlowControl|Switch|SwitchonETimelineDirection _direction
        (:Forward
          (Timeline|Oscillate PlayFromStart))
        (:Backward
          (Timeline|Oscillate ReverseFromEnd))))))

(fn ConstructionScript
  (|CallParentFunction))